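; Player stats component that tracks current and max health and stamina for the owning BP_ThirdPersonCharacter.
; BeginPlay caches the character and fills its HUD widget; each change function then pushes bar percentages, plus health text, straight to that widget.
; Increases to current values clamp at max, while decreases are unclamped.
; DecreaseHealth returns whether health is depleted; DecreaseStamina returns that same health check rather than testing stamina.
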(event `self.ReceiveBeginPlay`
  ;[0.7579 0 1] じゅうよう？？？
  (bind _asbp_third_person_character (cast `/Game/ThirdPerson/Blueprints/BP_ThirdPersonCharacter` (`self.GetOwner`)))
  (set `self.Player_Character_BP` _asbp_third_person_character)
  (`ProgressBar.SetPercent` (`/Game/0Contents/UI/WB_HUD.Health_Bar` (`/Game/ThirdPerson/Blueprints/BP_ThirdPersonCharacter.HUD_Widget` (`self.Player_Character_BP`))) (/ (`self.Current_Health`) (`self.Max_Health`)))
  (`TextBlock.SetText` (`/Game/0Contents/UI/WB_HUD.Health_Text` (`/Game/ThirdPerson/Blueprints/BP_ThirdPersonCharacter.HUD_Widget` (`self.Player_Character_BP`))) (`KismetTextLibrary.Conv_DoubleToText` (`self.Current_Health`) "HalfToEven"))
  (`ProgressBar.SetPercent` (`/Game/0Contents/UI/WB_HUD.Stamina_Bar` (`/Game/ThirdPerson/Blueprints/BP_ThirdPersonCharacter.HUD_Widget` (`self.Player_Character_BP`))) (/ (`self.Current_Stamina`) (`self.Max_Stamina`))))

(fn `Decrease_Health`
  (params (Damage :type "Float (double-precision)"))
  (returns (is_Player_Dead :type Boolean))
  ;[1 1 1] ないぶしょり　すうちせってい
  (bind _output_get (set `self.Current_Health` (- (`self.Current_Health`) Damage)))
  ;[1 1 1] ひょうじ
  ;;[1 1 1] うぃじぇっとの！すうちのせってい
  (`ProgressBar.SetPercent` (`/Game/0Contents/UI/WB_HUD.Health_Bar` (`/Game/ThirdPerson/Blueprints/BP_ThirdPersonCharacter.HUD_Widget` (`self.Player_Character_BP`))) (/ _output_get (`self.Max_Health`)))
  ;;[1 1 1] てきすとひょうじ
  (`TextBlock.SetText` (`/Game/0Contents/UI/WB_HUD.Health_Text` (`/Game/ThirdPerson/Blueprints/BP_ThirdPersonCharacter.HUD_Widget` (`self.Player_Character_BP`))) (`KismetTextLibrary.Conv_DoubleToText` (`self.Current_Health`) "HalfToEven"))
  ;[1 1 1] きゃらがいきてるかどうか
  (if (<= (`self.Current_Health`) 0.0)
    (return true)
    (else
      (return false))))

(fn `Decrease_Stamina`
  (params (Stammina_Depleted :type "Float (double-precision)"))
  (returns (No_Stamina :type Boolean))
  (bind _output_get (set `self.Current_Stamina` (- (`self.Current_Stamina`) Stammina_Depleted)))
  (`ProgressBar.SetPercent` (`/Game/0Contents/UI/WB_HUD.Stamina_Bar` (`/Game/ThirdPerson/Blueprints/BP_ThirdPersonCharacter.HUD_Widget` (`self.Player_Character_BP`))) (/ _output_get (`self.Max_Stamina`)))
  (if (<= (`self.Current_Health`) 0.0)
    (return true)
    (else
      (return false))))

(fn `Increase_Health`
  (params (Added_Health :type "Float (double-precision)"))
  (set `self.Current_Health` (+ (`self.Current_Health`) Added_Health))
  (if (> (`self.Current_Health`) (`self.Max_Health`))
    (set `self.Current_Health` (`self.Max_Health`)))
  (`ProgressBar.SetPercent` (`/Game/0Contents/UI/WB_HUD.Health_Bar` (`/Game/ThirdPerson/Blueprints/BP_ThirdPersonCharacter.HUD_Widget` (`self.Player_Character_BP`))) (/ (`self.Current_Health`) (`self.Max_Health`)))
  (`TextBlock.SetText` (`/Game/0Contents/UI/WB_HUD.Health_Text` (`/Game/ThirdPerson/Blueprints/BP_ThirdPersonCharacter.HUD_Widget` (`self.Player_Character_BP`))) (`KismetTextLibrary.Conv_DoubleToText` (`self.Current_Health`) "HalfToEven")))

(fn `Increase_Max_Health`
  (params (Max_Health_Value :type "Float (double-precision)"))
  (set `self.Max_Health` (+ (`self.Max_Health`) Max_Health_Value))
  (`ProgressBar.SetPercent` (`/Game/0Contents/UI/WB_HUD.Health_Bar` (`/Game/ThirdPerson/Blueprints/BP_ThirdPersonCharacter.HUD_Widget` (`self.Player_Character_BP`))) (/ (`self.Current_Health`) (`self.Max_Health`)))
  (`TextBlock.SetText` (`/Game/0Contents/UI/WB_HUD.Health_Text` (`/Game/ThirdPerson/Blueprints/BP_ThirdPersonCharacter.HUD_Widget` (`self.Player_Character_BP`))) (`KismetTextLibrary.Conv_DoubleToText` (`self.Current_Health`) "HalfToEven")))

(fn `Increase_Max_Stamina`
  (params (Added_Stamina :type "Float (double-precision)"))
  (set `self.Max_Stamina` (+ (`self.Max_Stamina`) Added_Stamina))
  (`ProgressBar.SetPercent` (`/Game/0Contents/UI/WB_HUD.Stamina_Bar` (`/Game/ThirdPerson/Blueprints/BP_ThirdPersonCharacter.HUD_Widget` (`self.Player_Character_BP`))) (/ (`self.Current_Stamina`) (`self.Max_Stamina`))))

(fn `Increase_Stamina`
  (params (B :type "Float (double-precision)"))
  (set `self.Current_Stamina` (+ (`self.Current_Stamina`) B))
  (if (> (`self.Current_Stamina`) (`self.Max_Stamina`))
    (bind _output_get (set `self.Current_Stamina` (`self.Max_Stamina`))))
  (`ProgressBar.SetPercent` (`/Game/0Contents/UI/WB_HUD.Stamina_Bar` (`/Game/ThirdPerson/Blueprints/BP_ThirdPersonCharacter.HUD_Widget` (`self.Player_Character_BP`))) (/ _output_get (`self.Max_Stamina`))))